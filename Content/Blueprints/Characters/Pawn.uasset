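; Lane-aware combat pawn that damages Frnd_Pawn actors entering its sphere.
; Capsule overlaps with front, mid and back lane actors set its Position enum.
; Incoming damage lowers Health with a one-second DoOnce cooldown, and death destroys it and shows HUD_Dialogue, while Tick updates the health bar.
; MoveByButton issues an AI move toward the first Pawn-class actor found, then a delayed move to a fixed point.
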(event OnComponentBeginOverlap(Sphere)
  (params (OverlappedComponent :type Primitive%20Component%20Object%20Reference) (OtherActor :type Actor%20Object%20Reference) (OtherComp :type Primitive%20Component%20Object%20Reference) (OtherBodyIndex :type Integer) (bFromSweep :type Boolean) (SweepResult :type Hit%20Result%20Structure%20%28by%20ref%29))
  (bind _asfrnd_pawn (Utilities|Casting|CastToFrnd_Pawn OtherActor))
  (Game|Damage|ApplyDamage _asfrnd_pawn 2e+01 0 0))

(event OnComponentBeginOverlap(CapsuleComponent)
  (params (OverlappedComponent :type Primitive%20Component%20Object%20Reference) (OtherActor :type Actor%20Object%20Reference) (OtherComp :type Primitive%20Component%20Object%20Reference) (OtherBodyIndex :type Integer) (bFromSweep :type Boolean) (SweepResult :type Hit%20Result%20Structure%20%28by%20ref%29))
  (Utilities|FlowControl|Sequence
    (:then_0
      (Utilities|Casting|CastToFrontLane3 OtherActor)
      (Variables|Default|SetPosition "NewEnumerator0" :!label _label))
    (:then_1
      (Utilities|Casting|CastToMidLane3 OtherActor)
      (Variables|Default|SetPosition "NewEnumerator2" :!label _label_2))
    (:then_2
      (Utilities|Casting|CastToBackLane3 OtherActor)
      (Variables|Default|SetPosition "NewEnumerator1" :!label _label_3))
    (:then_3
      (Utilities|Casting|CastToFrontLane1 OtherActor)
      (goto _label))
    (:then_4
      (Utilities|Casting|CastToFrontLane2 OtherActor)
      (goto _label))
    (:then_5
      (Utilities|Casting|CastToFrontLane1F OtherActor)
      (goto _label))
    (:then_6
      (Utilities|Casting|CastToFrontLane2F OtherActor)
      (goto _label))
    (:then_7
      (Utilities|Casting|CastToFrontLane3F OtherActor)
      (goto _label))
    (:then_8
      (Utilities|Casting|CastToMidLane1F OtherActor)
      (goto _label_2))
    (:then_9
      (Utilities|Casting|CastToMidLane2F OtherActor)
      (goto _label_2))
    (:then_10
      (Utilities|Casting|CastToMidLane3F OtherActor)
      (goto _label_2))
    (:then_11
      (Utilities|Casting|CastToMidLane1 OtherActor)
      (goto _label_2))
    (:then_12
      (Utilities|Casting|CastToMidLane2 OtherActor)
      (goto _label_2))
    (:then_13
      (Utilities|Casting|CastToBackLane1F OtherActor)
      (goto _label_3))
    (:then_14
      (Utilities|Casting|CastToBackLane2F OtherActor)
      (goto _label_3))
    (:then_15
      (Utilities|Casting|CastToBackLane3F OtherActor)
      (goto _label_3))
    (:then_16
      (Utilities|Casting|CastToBackLane1 OtherActor)
      (goto _label_3))
    (:then_17
      (Utilities|Casting|CastToBackLane2 OtherActor)
      (goto _label_3))))

(event Custom|MoveByButton
  (bind _self self)
  (bind _returnvalue (AI|GetAIController _self))
  (bind _returnvalue_2 (Actor|GetActorOfClass "Pawn_C"))
  (AI|AIMoveTo _returnvalue "0, 0, 0" _returnvalue_2 -1.0 "Default" "Default" true true
    (:then
      (Utilities|FlowControl|Delay 0.5)
      (AI|AIMoveTo _returnvalue (+ "" "9.000000,0.000000,0.000000") 0 -1.0 "Default" "Default" true true))))

(event Game|Damage|EventAnyDamage
  (params (Damage :type Float%20%28single-precision%29) (DamageType :type Damage%20Type%20Object%20Reference) (InstigatedBy :type Controller%20Object%20Reference) (DamageCauser :type Actor%20Object%20Reference))
  (Utilities|FlowControl|DoOnce false :!label _label
    (:Completed
      (bind _output_get (Variables|Default|SetHealth (- (Variables|Default|GetHealth) Damage)))
      (if (<= _output_get 0.0)
        (Actor|DestroyActor)
        (bind _returnvalue (UserInterface|CreateWidget "/Game/Blueprints/Hud/HUD_Dialogue.HUD_Dialogue_C"))
        (bind _output_get_2 (Variables|Default|SetNewVar _returnvalue))
        (UserInterface|Viewport|AddtoViewport _output_get_2 0)
        (else
          (Utilities|FlowControl|Delay 1.0)
          (goto _label Reset))))))

(event EventTick
  (params (DeltaSeconds :type Float%20%28single-precision%29))
  (bind _ashp_bar (Utilities|Casting|CastToHP_Bar (UserInterface|GetWidget (Variables|Default|GetWidget))))
  (Progress|SetPercent (Variables|/Game/Blueprints/Characters/HP_Bar.HP_Bar_C|GetHealthBar _ashp_bar) (/ (Variables|Default|GetHealth) 1e+02)))

(fn ConstructionScript)