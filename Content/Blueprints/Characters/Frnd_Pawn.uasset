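; Frnd_Pawn is an AI-moved pawn that makes a short move on command and damages pawns it touches.
; MoveByButton sends it toward the first Pawn found, then half a second after issuing that move, without waiting for arrival, redirects it near its stored spawn position.
; OnSpawn receives that start position, and the Sphere's begin overlap applies fixed damage to any overlapping Pawn.
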(event OnComponentBeginOverlap(Sphere)
  (params (OverlappedComponent :type Primitive%20Component%20Object%20Reference) (OtherActor :type Actor%20Object%20Reference) (OtherComp :type Primitive%20Component%20Object%20Reference) (OtherBodyIndex :type Integer) (bFromSweep :type Boolean) (SweepResult :type Hit%20Result%20Structure%20%28by%20ref%29))
  (bind _aspawn (Utilities|Casting|CastToPawn OtherActor))
  (Game|Damage|ApplyDamage _aspawn 2e+01 0 0 "/Script/Engine.DamageType"))

(event Custom|MoveByButton
  (bind _self self)
  (bind _returnvalue (AI|GetAIController _self))
  (bind _returnvalue_2 (Actor|GetActorOfClass "/Game/Blueprints/Characters/Pawn.Pawn_C"))
  (AI|AIMoveTo _returnvalue "0, 0, 0" _returnvalue_2 -1.0 "Default" "Default" true true
    (:then
      (Utilities|FlowControl|Delay 0.5)
      (AI|AIMoveTo _returnvalue (+ (Variables|Default|GetPosition%20Start) "9.000000,0.000000,0.000000") 0 -1.0 "Default" "Default" true true))))

(event Custom|OnSpawn
  (params (PositionStart :type Vector))
  (Variables|Default|SetPosition%20Start PositionStart))

(fn ConstructionScript)